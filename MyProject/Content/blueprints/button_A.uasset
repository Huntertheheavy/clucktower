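; Interactable button actor that toggles between pressed and unpressed states each time InteractFunc1 fires.
; Each toggle flips IsPressed, swaps the Cube's material between Bober_Mat and an empty slot, and calls the OnButtonPressed dispatcher so other objects can react.
; It also plays a door open or close sound cue to match the new state.
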(event EventBeginPlay)

(event Collision|EventActorBeginOverlap
  (params (OtherActor :type Actor%20Object%20Reference)))

(event EventTick
  (params (DeltaSeconds :type Float%20%28single-precision%29)))

(event EventInteractFunc1
  (params (Player :type BP%20First%20Person%20Character%20Object%20Reference))
  (if (Variables|Default|GetisPressed)
    (Rendering|Material|SetMaterial (Variables|Default|GetCube) 0 0)
    (Variables|Default|SetisPressed false)
    (Default|CallOnButtonPressed)
    (Audio|PlaySound2D "/Game/SFX/doorClose_Cue.doorClose_Cue" 1.0 1.0 0.0 0 0)
    (else
      (Rendering|Material|SetMaterial (Variables|Default|GetCube) 0 "/Game/Textures/bober_Mat.bober_Mat")
      (Variables|Default|SetisPressed true)
      (Default|CallOnButtonPressed)
      (Audio|PlaySound2D "/Game/SFX/doorOpen_Cue.doorOpen_Cue" 1.0 1.0 0.0 0 0))))

(fn ConstructionScript)
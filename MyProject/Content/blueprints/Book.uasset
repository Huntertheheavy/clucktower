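; Book actor that acts as a surveillance-camera viewer, with a widget-driven camera selector and a footage surface.
; On BeginPlay it passes all Camera_A actors to its Book_UMG widget, binds a switch event and activates the first map room's camera.
; A dynamic material shows that camera's render target.
; Swaps toggle a material scalar around a short delay, deactivating the previous camera and activating the new one.
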(event Custom|CE_SwapCamera
  (params (CameraARef :type Camera%20A%20Object%20Reference))
  (CallFunction|CamOff)
  (CallFunction|UpdateCamera CameraARef)
  (Utilities|FlowControl|Delay 0.1)
  (CallFunction|Camon))

(event EventBeginPlay
  (bind _asbook_umg (Utilities|Casting|CastToBook_UMG (UserInterface|GetWidget (Variables|Default|GetCameraHUD))))
  (bind _output_get (Variables|Default|SetBookUMG _asbook_umg))
  (EventDispatchers|BindEventtoSwitchCameraBook _output_get (EventDispatchers|CreateEvent :!event Custom|CE_SwapCamera))
  (bind _outactors (Actor|GetAllActorsOfClass "/Game/blueprints/Camera_A.Camera_A_C"))
  (Default|ImportCameras (Variables|Default|GetBookUMG) _outactors)
  (CallFunction|ActivateDefault))

(fn ConstructionScript
  (bind _returnvalue (Rendering|Material|CreateDynamicMaterialInstance (Variables|Default|GetFootage) 0 "/Game/Textures/Camera_Material.Camera_Material" "None" :!class /Script/Engine.PrimitiveComponent))
  (bind _output_get (Variables|Default|SetDynamicMaterialInstance _returnvalue))
  (Rendering|Material|SetMaterial (Variables|Default|GetFootage) 0 _output_get))

(fn ActivateDefault
  (bind _asroom_umg (Utilities|Casting|CastToRoom_UMG (Class|PanelWidget|GetChildat (Variables|/Game/blueprints/Book_UMG.Book_UMG_C|GetMap_CP (Variables|Default|GetBookUMG)))))
  (Default|SelectCamera _asroom_umg)
  (Variables|Default|SetPreviousCamera (Variables|/Game/blueprints/Room_UMG.Room_UMG_C|GetCameraRef _asroom_umg))
  (Default|CEActivateCamera (Variables|/Game/blueprints/Room_UMG.Room_UMG_C|GetCameraRef _asroom_umg))
  (Rendering|Material|SetTextureParameterValue (Variables|Default|GetDynamicMaterialInstance) "R" (Variables|/Script/Engine.SceneCaptureComponent2D|GetTextureTarget (Variables|/Game/blueprints/Camera_A.Camera_A_C|GetSceneCaptureComponent2D (Variables|/Game/blueprints/Room_UMG.Room_UMG_C|GetCameraRef _asroom_umg)))))

(fn UpdateCamera
  (params (NewCamera :type Camera%20A%20Object%20Reference))
  (bind _previouscamera (Variables|Default|GetPreviousCamera)
    (:then
      (Default|CEDeactivate _previouscamera)
      (bind _output_get (Variables|Default|SetPreviousCamera NewCamera))
      (Default|CEActivateCamera _output_get))
    (:else)))

(fn CamOff
  (Rendering|Material|SetScalarParameterValue (Variables|Default|GetDynamicMaterialInstance) "Deactivate" 0.0 :!class /Script/Engine.MaterialInstanceDynamic))

(fn Camon
  (Rendering|Material|SetScalarParameterValue (Variables|Default|GetDynamicMaterialInstance) "Deactivate" 1.0 :!class /Script/Engine.MaterialInstanceDynamic))